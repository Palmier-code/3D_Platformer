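; Rifle test actor that automatically fires a hitscan shot on a looping half-second timer from BeginPlay.
; Each shot runs a persistent debug-drawn visibility trace from the actor's location to its forward vector times Range, without adding that location to the end point.
; It spawns an explosion emitter at the hit location and prints whether the hit actor is a ThirdPersonCharacter, without applying damage.
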(event Custom|Fire
  (bind _outhit (Collision|LineTraceByChannel (Transformation|GetActorLocation) (* (Transformation|GetActorForwardVector) (Variables|Default|GetRange)) "TraceTypeQuery1" false 0 "Persistent"))
  (Effects|SpawnEmitteratLocation "/Game/StarterContent/Particles/P_Explosion.P_Explosion" (.location _outhit))
  (Utilities|Casting|CastToThirdPersonCharacter (.hitactor _outhit)
    (:then
      (Development|PrintString "toucher"))
    (:CastFailed
      (Development|PrintString "fail"))))

(event EventBeginPlay
  (Utilities|Time|SetTimerbyEvent (delegate Custom|Fire) 0.5 true))

(event Collision|EventActorBeginOverlap
  (params (OtherActor :type Actor%20Object%20Reference)))

(event EventTick
  (params (DeltaSeconds :type Float%20%28single-precision%29)))

(fn ConstructionScript)